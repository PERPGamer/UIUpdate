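; Revive controller component that manages the updated wounded screen UI for a player controller.
; LoadWoundedScreen creates the revive widget once for the owning controller.
; WoundedScreenToggle adds it to the player screen with a forward animation, or zeroes its panel opacity and removes it.
; Each actual change in visibility records the shown state and hides the HUD while the wounded screen is up, restoring it afterwards.
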(fn `LoadWoundedScreen`
  (`/Engine/EditorBlueprintResources/StandardMacros.IsValid` (`self.NewWoundedScreen`)
    (:`Is Not Valid`
      (bind _returnvalue (`|CreateWidget` "/UIUpdate/UI/Interaction/WBP_WoundedScreenRevive_UIUpdate.WBP_WoundedScreenRevive_UIUpdate_C" (`self.Controller`)))
      (set `self.NewWoundedScreen` _returnvalue))))

(fn `WoundedScreenToggle`
  (params (Show :type Boolean))
  (locals (bWoundedScreenShown :type Boolean))
  (bind _newwoundedscreen (`self.NewWoundedScreen`))
  (bind _newwoundedscreen_2 (`self.NewWoundedScreen`))
  (bind _returnvalue (`Widget.IsInViewport` _newwoundedscreen_2))
  (`/Engine/EditorBlueprintResources/StandardMacros.IsValid` _newwoundedscreen_2
    (:`Is Valid`
      (if (`local.Show`)
        (if (not _returnvalue)
          (`UserWidget.AddToPlayerScreen` _newwoundedscreen 0)
          (`UserWidget.PlayAnimationForward` _newwoundedscreen (`/UIUpdate/UI/Interaction/WBP_WoundedScreenRevive_UIUpdate.NewAnimation_1` _newwoundedscreen) 1.0 false)
          (bind _output_get (set `local.bWoundedScreenShown` (`local.Show`) :!label _label))
          (if _output_get
            (`/HDCore/Core/BP_HDPlayerControllerBase.HideHUD` (`self.Controller`))
            (else
              (`/HDCore/Core/BP_HDPlayerControllerBase.ShowHUD` (`self.Controller`)))))
        (elif _returnvalue
          (`Widget.SetRenderOpacity` (`/UIUpdate/UI/Interaction/WBP_WoundedScreenRevive_UIUpdate.WoundedPanel` _newwoundedscreen) 0.0)
          (`Widget.RemoveFromParent` (`self.NewWoundedScreen`))
          (goto _label))))))
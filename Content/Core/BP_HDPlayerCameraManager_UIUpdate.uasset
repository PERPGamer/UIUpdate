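; Player camera manager that hides the initial view and computes screen-space corrections for scope lens distortion.
; Construction fades to black and mutes SFX and Voice sound classes until OnReset restores them.
; ProjectWorldToScreenEx manually projects world points through the first-person camera's view-projection matrix at 1:1 aspect.
; CalculateLensDistortionTranslation turns that projection into an offset scaled by aim alpha and distortion, fading beyond the scope radius and skipped at aiming FOV 80+.
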(event `self.ReceiveBeginPlay`
  (`parent.ReceiveBeginPlay`))

(event `OnReset`
  (`self.StopCameraOverride`))

(fn `Calculate Lens Distortion Translation`
  (params (WorldPosition :type "Vector Structure") (Pawn :type "Pawn Object Reference"))
  (returns (Translation :type "Vector2D Structure") (Valid :type Boolean))
  (bind (_screenposition _screennormal _returnvalue) (`self.ProjectWorldToScreenEx` WorldPosition))
  (bind _returnvalue_2 (/ (`self.ScopeRadius`) (`self.ScopeRadiusDivider`)))
  (bind _returnvalue_3 (- _screennormal (0.5 0.5)))
  (bind _asbp_hdplayer_camera_manager_uiupdate (cast `/Game/Core/BP_HDPlayerCameraManager_UIUpdate` (`GameplayStatics.GetPlayerCameraManager` 0) :!pure true))
  (bind _returnvalue_4 (`KismetMathLibrary.VSize2D` _returnvalue_3))
  (bind _lensdistortionamount (`/Game/Core/BP_HDPlayerCameraManager_UIUpdate.LensDistortionAmount` _asbp_hdplayer_camera_manager_uiupdate))
  (bind _asbp_hdplayer_character_uiupdate (cast `/UIUpdate/Core/BP_HDPlayerCharacter_UIUpdate` Pawn))
  (bind _aimalpha (`/HDCore/Core/BP_HDPlayerCharacterBase.AimAlpha` _asbp_hdplayer_character_uiupdate))
  (if (and (> _aimalpha 0.0) (< (`DFPlayerCameraManager.AimingFOV` _asbp_hdplayer_camera_manager_uiupdate) 80.0) (!= _lensdistortionamount 0.0))
    (if (< _returnvalue_4 _returnvalue_2)
      (bind _returnvalue_5 (* _returnvalue_3 (* _aimalpha (* (`KismetMathLibrary.Abs` _lensdistortionamount) (`self.LensDistortionMultiplier`)))))
      (return _returnvalue_5 _returnvalue)
      (else
        (return (`/UIUpdate/Core/Libraries/FL_Core_UiUpdate.LerpVector2D` _returnvalue_5 (0.0 0.0) (`KismetMathLibrary.FClamp` (* (- _returnvalue_4 _returnvalue_2) (`self.ScopeEdgeFadeMultiplier`)))) _returnvalue)))
    (else
      (return (0.0 0.0) false))))

(fn `ProjectWorldToScreenEx`
  (params (WorldPosition :type "Vector Structure") (ConstrainAspectRatio :type Boolean) (OverrideFOV :type "Float (double-precision)"))
  (returns (ScreenPosition :type "Vector2D Structure") (ScreenNormal :type "Vector2D Structure") (ReturnValue :type Boolean))
  (bind _returnvalue (`GameplayStatics.GetPlayerController` 0))
  (bind (_sizex _sizey) (`PlayerController.GetViewportSize` (`GameplayStatics.GetPlayerController` 0)))
  (`/Engine/EditorBlueprintResources/StandardMacros.IsValid` _returnvalue
    (:`Is Valid`
      (bind _ashdplayer_character (cast `HDPlayerCharacter` (`Controller.K2_GetPawn` _returnvalue)))
      (bind _desiredview (`CameraComponent.GetCameraView` (`DFBasePlayerCharacter.GetCamera1P` _ashdplayer_character) 0.0))
      (setmembers `MinimalViewInfo` :`StructRef` _desiredview :`FOV` (`KismetMathLibrary.SelectFloat` OverrideFOV (`self.GetFOVAngle`) (> OverrideFOV 0.0)) :`AspectRatio` 1.0 :`bConstrainAspectRatio` false :!pinned true) ; NOTE: Aspect Ratio 1.0
      (bind (_x _y _z _w) (`KismetMathLibrary.BreakVector4` (`KismetMathLibrary.TransformVector4` (`.ViewProjectionMatrix` (`GameplayStatics.GetViewProjectionMatrix` _desiredview)) (`KismetMathLibrary.MakeVector4` (.x WorldPosition) (.y WorldPosition) (.z WorldPosition) 1.0))))
      (bind (_w_2 _x_2 _y_2) (break `Plane` (make `Plane` _w (.x (* (`KismetMathLibrary.MakeVector` _x _y _z) (/ 1.0 _w))) (.y (* (`KismetMathLibrary.MakeVector` _x _y _z) (/ 1.0 _w))) (.z (* (`KismetMathLibrary.MakeVector` _x _y _z) (/ 1.0 _w))))))
      (bind _returnvalue_2 (`KismetMathLibrary.MakeVector2D` (+ (/ _x_2 2.0) 0.5) (- (- 1.0 (/ _y_2 2.0)) 0.5)))
      (return (* (`KismetMathLibrary.MakeVector2D` (`KismetMathLibrary.Conv_IntToDouble` _sizex) (`KismetMathLibrary.Conv_IntToDouble` _sizey)) _returnvalue_2) _returnvalue_2 (> _w 0.0)))))

(fn `StartCameraOverride`
  (`self.SetManualCameraFade` 1.0)
  (`GameplayStatics.SetSoundMixClassOverride` "/HDCore/Core/SoundMixes/SM_Master.SM_Master" "/Engine/EngineSounds/SFX.SFX" 0.0 1.0 0.0) ; Disable world SFX till we spawn in for the first time
  (`GameplayStatics.SetSoundMixClassOverride` "/HDCore/Core/SoundMixes/SM_Master.SM_Master" "/Engine/EngineSounds/Voice.Voice" 0.0 1.0 0.0) ; Disable world voice till we spawn in for the first time
)

(fn `StopCameraOverride`
  (`self.StopCameraFade`)
  (`GameplayStatics.SetSoundMixClassOverride` "/HDCore/Core/SoundMixes/SM_Master.SM_Master" "/Engine/EngineSounds/SFX.SFX" 1.0 1.0 0.0) ; Re-enable world SFX
  (`GameplayStatics.SetSoundMixClassOverride` "/HDCore/Core/SoundMixes/SM_Master.SM_Master" "/Engine/EngineSounds/Voice.Voice" 1.0 1.0 0.0) ; Re-enable world voice
)

(fn `UserConstructionScript`
  (`parent.UserConstructionScript`)
  (`self.StartCameraOverride`))
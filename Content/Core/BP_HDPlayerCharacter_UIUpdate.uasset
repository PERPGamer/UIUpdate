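; Player character subclass for the HD UI update, keeping the HUD's magazine tray in sync with the equipped weapon's ammo.
; BeginPlay forces a reset on the custom camera manager as a workaround.
; UpdateMags rebuilds the tray, only where cosmetic events can run, on weapon change, fire and reload.
; A Tick hack also compares total ammo to the last value to catch ammo received from other players.
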(event `self.ReceiveBeginPlay`
  (`parent.ReceiveBeginPlay`)
  ;[1 0 0] Hack to get camera manager to work
  (bind _asbp_hdplayer_camera_manager_uiupdate (cast `/UIUpdate/Core/BP_HDPlayerCameraManager_UIUpdate` (`GameplayStatics.GetPlayerCameraManager` 0)))
  (`/UIUpdate/Core/BP_HDPlayerCameraManager_UIUpdate.OnReset` _asbp_hdplayer_camera_manager_uiupdate))

(event `self.ReceiveTick`
  (params (DeltaSeconds :type "Float (single-precision)"))
  (`parent.ReceiveTick` DeltaSeconds)
  ;[1 0 0] HACK to get ammo to update whenever you get ammo from another user
  (bind _equippedweapon (`self.EquippedWeapon`)
    (:`then`
      (if (!= (`DFBaseGun.GetTotalAmmo` _equippedweapon false) (`self.LastAmmo`))
        (set `self.LastAmmo` (`DFBaseGun.GetTotalAmmo` (`self.EquippedWeapon`) false))
        (`self.UpdateMags`)))
    (:`else`)))

(event `self.ReceiveEquippedItemChanged`
  (params (NewEquippedItem :type "DFBaseItem Object Reference") (PrevEquippedItem :type "DFBaseItem Object Reference"))
  (bind _equippedweapon (`self.EquippedWeapon`))
  (`parent.ReceiveEquippedItemChanged` NewEquippedItem PrevEquippedItem)
  (add `DFBaseGun.OnReloadFinished` _equippedweapon (`|CreateDelegate` :!event `OnReload`))
  (add `DFBaseWeapon.OnFire` _equippedweapon (`|CreateDelegate` :!event `OnFire`))
  (`self.UpdateMags`))

(event `OnFire`
  (params (FiredWeapon :type "DFBaseWeapon Object Reference") (bLastFire :type Boolean))
  ;[1 0 0] Hacky way of updating mags
  (`self.UpdateMags`))

(event `OnReload`
  (params (Gun :type "DFBaseGun Object Reference"))
  ;[1 0 0] Hacky way of updating mags
  (`self.UpdateMags`))

(fn `UpdateMags`
  (`/Engine/EditorBlueprintResources/StandardMacros.Can Execute Cosmetic Events`
    (:`True`
      (bind _asbp_hdhud_uiupdate (cast `/UIUpdate/Core/BP_HDHUD_UIUpdate` (`/HDCore/Core/BPFL_HDCore.GetHDHUDBP` 0)))
      (bind _aswbp_huduiupdate (cast `/UIUpdate/UI/HUD/WBP_HUDUIUpdate` (`/HDCore/Core/BP_HDHUDBase.GetValidCharacterHUDContainer` _asbp_hdhud_uiupdate)))
      (`/UIUpdate/UI/HUD/AmmoCount/WBP_MagTray.Create Mags` (`/UIUpdate/UI/HUD/WeaponStatus/WBP_WeaponStatus_UIUpdate.MagTray` (`/UIUpdate/UI/HUD/WBP_HUDUIUpdate.WeaponStatus_UI` _aswbp_huduiupdate))))))

(fn `UserConstructionScript`
  (`parent.UserConstructionScript`))
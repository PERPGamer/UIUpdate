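; Player controller variant that swaps in the UI-update deploy menu and death screen widgets and returns a child revive controller component.
; Deploy menu and death screen overrides create, preload or show their widgets, toggling the HUD and exposing the spawn map's minimap.
; On BeginPlay, a cosmetic-only hack hides and replaces every capture point's icon widget before calling the parent.
; Tick edge-detects vehicle occupancy to fire enter and exit vehicle events.
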(event `self.ReceiveBeginPlay`
  (`|ExecutionSequence`
    (:`then_0`
      ;[1 0 0] Hack to replace Capture point UI
      (`/Engine/EditorBlueprintResources/StandardMacros.Can Execute Cosmetic Events`
        (:`True`
          (bind _outactors (`GameplayStatics.GetAllActorsOfClass` "/HDCore/Placeables/BP_HDCapturePointBase.BP_HDCapturePointBase_C"))
          (for _array_element _outactors
            (`Widget.SetRenderOpacity` (`WidgetComponent.GetUserWidgetObject` (`/HDCore/Placeables/BP_HDCapturePointBase.IconWidget` _array_element)) 0.0)
            (bind _returnvalue (`AddComponent|NODE_AddWidgetComponent-3` :`self` _array_element))
            (set `/HDCore/Placeables/BP_HDCapturePointBase.IconWidget` _returnvalue _array_element)))))
    (:`then_1`
      (`parent.ReceiveBeginPlay`))))

(event `self.ReceiveTick`
  (params (DeltaSeconds :type "Float (single-precision)"))
  (`parent.ReceiveTick` DeltaSeconds)
  (if (`self.IsInVehicle`)
    (if (not (`self.HasEnteredVehicle`))
      (`self.OnEnterVehicle`)
      (set `self.HasEnteredVehicle` true))
    (elif (`self.HasEnteredVehicle`)
      (`self.OnExitVehicle`)
      (set `self.HasEnteredVehicle` false))))

(fn `DeathScreenToggle`
  (params (bShow :type Boolean))
  (bind _deathscreen (`self.DeathScreen`))
  (bind _deathscreen_2 (`self.DeathScreen`))
  (bind _returnvalue (`Widget.IsInViewport` _deathscreen))
  (bind _aswbp_death_screen_uiupdate (cast `/UIUpdate/UI/Interaction/WBP_DeathScreen_UIUpdate` _deathscreen_2 :!pure true))
  (`/Engine/EditorBlueprintResources/StandardMacros.IsValid` _deathscreen
    (:`Is Valid`
      (if (`local.bShow`)
        (if (not _returnvalue)
          (`UserWidget.AddToPlayerScreen` _deathscreen_2 0)
          (`UserWidget.PlayAnimationForward` _deathscreen_2 (`/UIUpdate/UI/Interaction/WBP_DeathScreen_UIUpdate.DeathScreenFade` _aswbp_death_screen_uiupdate) 1.0 false)
          (bind _output_get (set `self.bDeathScreenShown` (`local.bShow`) :!label _label))
          (if _output_get
            (`self.HideHUD`)
            (else
              (`self.ShowHUD`))))
        (elif _returnvalue
          (`Widget.SetRenderOpacity` (`/UIUpdate/UI/Interaction/WBP_DeathScreen_UIUpdate.DeathScreenText` _aswbp_death_screen_uiupdate) 0.0)
          (`Widget.RemoveFromParent` (`self.DeathScreen`))
          (goto _label))))))

(fn `GetMinimapWidget`
  (returns (MinimapWidget :type "DFMinimap Object Reference"))
  (bind _deploymenu (`self.DeployMenu`)
    (:`then`
      (bind _aswbp_deploy_menu_uiupdate (cast `/UIUpdate/UI/DeployMenu/WBP_DeployMenu_UIUpdate` _deploymenu))
      (bind _spawnmapview (`/HDCore/UI/DeployMenu/WBP_DeployMenu.SpawnMapView` _aswbp_deploy_menu_uiupdate)
        (:`then`
          (return (`/HDCore/UI/DeployMenu/SpawnMap/WBP_DeployMenu_SpawnMapView.Minimap` _spawnmapview)))
        (:`else`)))
    (:`else`)))

(fn `GetReviveController`
  (returns (ReviveController :type "/HDCore/Core/Medical/BP_HDReviveControllerComponent Object Reference"))
  (return (`self.BP_HDReviveControllerComponent_Child`)))

(fn `LoadAndActivateDeployMenu`
  (locals (NewLocalVar_0 :type "PanelWidget Object Reference"))
  (bind _returnvalue (`DFMenuManagerBlueprintFunctions.CreateAndActivate` "/UIUpdate/UI/DeployMenu/WBP_DeployMenu_UIUpdate.WBP_DeployMenu_UIUpdate_C" self "Exclusive"))
  (set `self.DeployMenu` _returnvalue)
  (set `self.bDeployMenuShown` true)
  (`self.HideHUD`)
  (`HDGameInstance.UnloadScoreboardMenu` (cast `HDGameInstance` (`GameplayStatics.GetGameInstance`) :!pure true)))

(fn `LoadDeathScreen`
  (`/Engine/EditorBlueprintResources/StandardMacros.IsValid` (`self.DeathScreen`)
    (:`Is Not Valid`
      (bind _returnvalue (`|CreateWidget` "/UIUpdate/UI/Interaction/WBP_DeathScreen_UIUpdate.WBP_DeathScreen_UIUpdate_C" self))
      (set `self.DeathScreen` _returnvalue))))

(fn `LoadDeployMenu`
  (bind _returnvalue (`|CreateWidget` "/UIUpdate/UI/DeployMenu/WBP_DeployMenu_UIUpdate.WBP_DeployMenu_UIUpdate_C" self null null))
  (bind _output_get (set `self.DeployMenu` _returnvalue)) ; Store widget reference
  (add `/HDCore/UI/DeployMenu/WBP_DeployMenu.OnPreloadFinished` _output_get (`|CreateDelegate` :!event `OnDeployMenuPreloadFinished`))
  (`/HDCore/UI/DeployMenu/WBP_DeployMenu.PreloadContent` (`self.DeployMenu`)))

(fn `UserConstructionScript`
  (`parent.UserConstructionScript`))